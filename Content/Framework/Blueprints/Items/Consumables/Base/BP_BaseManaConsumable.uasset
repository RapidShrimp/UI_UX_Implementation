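; BP_BaseManaConsumable is a base consumable item that restores mana to the character who uses it.
; ConsumeEffect compares CurrentMana to MaxMana on the character's BPCAttributes component and, when below max, calls ModifyMana to add ManaUpdateAmount.
; It returns true when mana was added and false when mana is already full.
; The event graph holds only disabled default events.
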(fn `ConsumeEffect`
  (params (ConsumingCharacter :type "/Game/Framework/Blueprints/Characters/BP_BaseCharacter Object Reference"))
  (returns (`Success?` :type Boolean))
  (bind _bpc_attributes (`/Game/Framework/Blueprints/Characters/BP_BaseCharacter.BPC_Attributes` ConsumingCharacter))
  (bind ((`CurrentMana_6_8E9069F34D25BFE011302DA22DA74FCC` _currentmana) (`MaxMana_8_D5F3680A407EE725F74AD98604258589` _maxmana)) (break `/Game/Framework/Blueprints/Data/Attributes/Struct_GameplayAttributes` (`/Game/Framework/Blueprints/Components/BPC_Attributes.GameplayAttributes` _bpc_attributes)))
  (if (< _currentmana _maxmana)
    (`/Game/Framework/Blueprints/Components/BPC_Attributes.ModifyMana` _bpc_attributes true (`self.ManaUpdateAmount`))
    (return true)
    (else
      (return false))))

(fn `UserConstructionScript`
  (`parent.UserConstructionScript`))