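; Base item Blueprint that provides shared use and rarity-highlight functions driven by its ItemData.
; UseItem prints the item's name as a used-item message and returns true, without acting on the using character.
; SetRarityColour maps the five rarity tiers from Common to Legendary onto an integer highlight value.
; Initialise and the construction script are empty.
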(fn `Initialise`)

(fn `SetRarityColour`
  (returns (HighlightValue :type Integer))
  (bind _output_get (set `self.RarityHighlightValue` (select `/Game/Framework/Blueprints/Data/Items/Enum_ItemRarity` (`.ItemRarity_46_D48462DC446B4F9CB1F49D916990066E` (break `/Game/Framework/Blueprints/Data/Items/Struct_ItemData` (`self.ItemData`))) :`NewEnumerator0` 1 :`NewEnumerator1` 2 :`NewEnumerator2` 3 :`NewEnumerator3` 4 :`NewEnumerator4` 5)))
  (return _output_get))

(fn `UseItem`
  (params (UsingCharacter :type "/Game/Framework/Blueprints/Characters/BP_BaseCharacter Object Reference"))
  (returns (`bSuccess?` :type Boolean))
  (set `self.Using Character` UsingCharacter)
  (`KismetSystemLibrary.PrintString` (`KismetStringLibrary.Concat_StrStr` "Player used Item : " (`KismetTextLibrary.Conv_TextToString` (`.ItemName_2_F7BAC0A2440EBA0D7C3512BA5436157F` (break `/Game/Framework/Blueprints/Data/Items/Struct_ItemData` (`self.ItemData`))))))
  (return true))

(fn `UserConstructionScript`)