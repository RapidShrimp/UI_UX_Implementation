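; Base class for equipment items, where using the item toggles it between equipped and unequipped on the using character.
; UseItem calls RemoveItem or EquipItem on the character's BPCEquipment component and updates the Equipped flag from the returned result.
; It then calls the parent UseItem and returns its result, printing debug strings along the way.
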(fn `UseItem`
  (params (UsingCharacter :type "/Game/Framework/Blueprints/Characters/BP_BaseCharacter Object Reference"))
  (returns (`bSuccess?` :type Boolean))
  (locals (LocalUsingCharacter :type "/Game/Framework/Blueprints/Characters/BP_BaseCharacter Object Reference"))
  (bind _output_get (set `local.LocalUsingCharacter` UsingCharacter))
  (if (`self.Equipped?`)
    (bind _bpc_equipment (`/Game/Framework/Blueprints/Characters/BP_BaseCharacter.BPC_Equipment` _output_get))
    (bind _success_ (`/Game/Framework/Blueprints/Components/BPC_Equipment.RemoveItem` _bpc_equipment self))
    ;[0 0 0] Debug
    (`KismetSystemLibrary.PrintString` (`KismetStringLibrary.Concat_StrStr` "Remove the Item is " (`KismetStringLibrary.Conv_BoolToString` _success_)))
    (set `self.Equipped?` (not _success_))
    (else
      ;[0 0 0] Debug
      (`KismetSystemLibrary.PrintString` (`KismetStringLibrary.Concat_StrStr` "Equipping Item : " (`KismetSystemLibrary.GetDisplayName` self)))
      (bind _success__2 (`/Game/Framework/Blueprints/Components/BPC_Equipment.EquipItem` _bpc_equipment self))
      (set `self.Equipped?` _success__2)))
  (bind _bsuccess_ (`parent.UseItem` (`local.LocalUsingCharacter`)))
  (return _bsuccess_))

(fn `UserConstructionScript`
  (`parent.UserConstructionScript`))