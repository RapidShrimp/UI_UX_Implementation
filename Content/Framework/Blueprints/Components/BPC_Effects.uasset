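; Actor component that manages the buff and debuff effects on its owning character.
; AddEffect spawns each effect as an actor and sorts it into Buffs or Debuffs by type.
; If one of the same class is already active, the new actor is destroyed and the existing one gains a stack.
; Event dispatchers announce additions, endings and refreshes, while HandleEffectEnding removes and destroys finished effects.
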(event `/Game/Framework/Blueprints/Interfaces/BPI_Effects.ApplyNewEffect`
  (params (EffectsToAdd :type "/Game/Framework/Blueprints/Effects/Base/BP_BaseEffect Class Reference"))
  (`self.Add Effect` EffectsToAdd))

(fn `Add Effect`
  (params (EffectsToAdd :type "/Game/Framework/Blueprints/Effects/Base/BP_BaseEffect Class Reference"))
  (locals (LocalEffect :type "/Game/Framework/Blueprints/Effects/Base/BP_BaseEffect Object Reference"))
  (bind _localeffect (`local.LocalEffect`))
  (bind _localeffect_2 (`local.LocalEffect`))
  (bind _returnvalue (`|SpawnActorFromClass` EffectsToAdd (`KismetMathLibrary.MakeTransform` (0.0 0.0 0.0)) "Undefined" "SelectDefaultAtRuntime" null (`self.Owning Character`)))
  (`/Game/Framework/Blueprints/Effects/Base/BP_BaseEffect.Initialise` _returnvalue (`self.Owning Character`))
  (bind _output_get (set `local.LocalEffect` _returnvalue))
  (bind _outeffect (`self.DoesEffectExist` _output_get))
  (`/Engine/EditorBlueprintResources/StandardMacros.IsValid` _outeffect
    (:`Is Valid`
      (`Actor.K2_DestroyActor` (`local.LocalEffect`))
      (bind _output_get_2 (set `local.LocalEffect` _outeffect))
      (`/Game/Framework/Blueprints/Effects/Base/BP_BaseEffect.AddStack` _output_get_2))
    (:`Is Not Valid`
      (switch `/Game/Framework/Blueprints/Data/Effects/Enum_EffectTypes` (`.EffectType_14_037EC23F468B25787FD3A099EFBF03B2` (break `/Game/Framework/Blueprints/Data/Effects/Struct_EffectData` (`/Game/Framework/Blueprints/Effects/Base/BP_BaseEffect.EffectData` _localeffect)))
        (:`NewEnumerator0`
          (`KismetArrayLibrary.Array_Add` (`self.Buffs`) _localeffect))
        (:`NewEnumerator1`
          (`KismetArrayLibrary.Array_Add` (`self.Debuffs`) _localeffect)))
      (add `/Game/Framework/Blueprints/Effects/Base/BP_BaseEffect.E_EndEffect` _localeffect_2 (`|CreateDelegate` :!event `HandleEffectEnding`))
      (`/Game/Framework/Blueprints/Effects/Base/BP_BaseEffect.StartEffect` _localeffect_2)
      (`self.E_AddEffect` (`local.LocalEffect`))))
  (`self.E_RefreshEffects`))

(fn `DoesEffectExist`
  (params (IncomingEffect :type "/Game/Framework/Blueprints/Effects/Base/BP_BaseEffect Object Reference"))
  (returns (OutEffect :type "/Game/Framework/Blueprints/Effects/Base/BP_BaseEffect Object Reference"))
  (locals (LocalEffectToFind :type "/Game/Framework/Blueprints/Effects/Base/BP_BaseEffect Object Reference") (TempArray :type "Array of /Game/Framework/Blueprints/Effects/Base/BP_BaseEffect Object Reference") (LocalEffectToReturn :type "/Game/Framework/Blueprints/Effects/Base/BP_BaseEffect Object Reference"))
  (bind _output_get (set `local.LocalEffectToFind` IncomingEffect))
  (switch `/Game/Framework/Blueprints/Data/Effects/Enum_EffectTypes` (`.EffectType_14_037EC23F468B25787FD3A099EFBF03B2` (break `/Game/Framework/Blueprints/Data/Effects/Struct_EffectData` (`/Game/Framework/Blueprints/Effects/Base/BP_BaseEffect.EffectData` _output_get)))
    (:`NewEnumerator0`
      (set `local.TempArray` (`self.Buffs`)))
    (:`NewEnumerator1`
      (set `local.TempArray` (`self.Debuffs`))))
  (for _array_element (`local.TempArray`)
    (if (== (`GameplayStatics.GetObjectClass` _array_element) (`GameplayStatics.GetObjectClass` (`local.LocalEffectToFind`)))
      (set `local.LocalEffectToReturn` _array_element)
      (break)))
  (return (`local.LocalEffectToReturn`)))

(fn `HandleEffectEnding`
  (params (EndingEffect :type "/Game/Framework/Blueprints/Effects/Base/BP_BaseEffect Object Reference"))
  (locals (LocalEndingEffect :type "/Game/Framework/Blueprints/Effects/Base/BP_BaseEffect Object Reference"))
  (bind ((`EffectName_2_D6DC489244E527F5002982B905FED353` _effectname)) (break `/Game/Framework/Blueprints/Data/Effects/Struct_EffectData` (`/Game/Framework/Blueprints/Effects/Base/BP_BaseEffect.EffectData` (`local.LocalEndingEffect`))))
  (bind _output_get (set `local.LocalEndingEffect` EndingEffect))
  (switch `/Game/Framework/Blueprints/Data/Effects/Enum_EffectTypes` (`.EffectType_14_037EC23F468B25787FD3A099EFBF03B2` (break `/Game/Framework/Blueprints/Data/Effects/Struct_EffectData` (`/Game/Framework/Blueprints/Effects/Base/BP_BaseEffect.EffectData` _output_get)))
    (:`NewEnumerator0`
      (`KismetArrayLibrary.Array_RemoveItem` (`self.Buffs`) (`local.LocalEndingEffect`))
      (`self.E_EffectEnded` _effectname true))
    (:`NewEnumerator1`
      (`KismetArrayLibrary.Array_RemoveItem` (`self.Debuffs`) (`local.LocalEndingEffect`))
      (`self.E_EffectEnded` _effectname)))
  (`Actor.K2_DestroyActor` (`local.LocalEndingEffect`))
  (`self.E_RefreshEffects`))

(fn `Initialise`
  (params (OwningCharacter :type "/Game/Framework/Blueprints/Characters/BP_BaseCharacter Object Reference"))
  (set `self.Owning Character` OwningCharacter))