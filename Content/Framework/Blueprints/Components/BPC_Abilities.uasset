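; Ability component that spawns and manages a character's abilities and handles requests to use them.
; Initialise spawns an actor for each configured ability class, initialises it with the owner and its index, and stores it.
; UseAbility looks up an ability by index, checks cooldown and the owner's current mana, then starts the cast.
; Event calls report successful use, both failure reasons and cooldown completion.
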(fn `AbilityCooledDown`
  (params (Ability :type "/Game/Framework/Blueprints/Abilities/Base/BP_BaseAbility Object Reference"))
  (`self.E_AbilityReady` Ability))

(fn `Initialise`
  (params (OwningCharacter :type "/Game/Framework/Blueprints/Characters/BP_BaseCharacter Object Reference"))
  (set `self.Owning Character` OwningCharacter)
  (for (_array_element _array_index) (`self.AbilitiesToSpawn`)
    (bind _returnvalue (`|SpawnActorFromClass` _array_element (`KismetMathLibrary.MakeTransform` (0.0 0.0 0.0)) "Undefined" "SelectDefaultAtRuntime" null null))
    (`/Game/Framework/Blueprints/Abilities/Base/BP_BaseAbility.Initialise` _returnvalue (`self.Owning Character`) _array_index)
    (`KismetArrayLibrary.Array_AddUnique` (`self.AbilityRef`) _returnvalue)))

(fn `UseAbility`
  (params (Index :type Integer))
  (returns (Success :type Boolean))
  (locals (LocalAbility :type "/Game/Framework/Blueprints/Abilities/Base/BP_BaseAbility Object Reference"))
  (bind _localability (`local.LocalAbility`))
  (bind _output_get (set `local.LocalAbility` (`|GetArrayItem` (`self.AbilityRef`) Index)))
  (`/Engine/EditorBlueprintResources/StandardMacros.IsValid` _output_get
    (:`Is Valid`
      (bind ((`ManaCost_9_ED8622F44C9BB2B067A4AEB193B018C4` _manacost) (`OnCooldown_14_05A44E6C4479C8C6DD247DB54A60EB4A` _oncooldown)) (break `/Game/Framework/Blueprints/Data/Ability/Struct_AbilityData` (`/Game/Framework/Blueprints/Abilities/Base/BP_BaseAbility.AbilityData` _output_get)))
      (if _oncooldown
        (`self.E_FailedAbilityOnCooldown`)
        (`KismetSystemLibrary.PrintString` "Use Ability Failed: On Cooldown")
        (return false)
        (elif (>= (- (`.CurrentMana_6_8E9069F34D25BFE011302DA22DA74FCC` (break `/Game/Framework/Blueprints/Data/Attributes/Struct_GameplayAttributes` (`/Game/Framework/Blueprints/Components/BPC_Attributes.GameplayAttributes` (`/Game/Framework/Blueprints/Characters/BP_BaseCharacter.BPC_Attributes` (`self.Owning Character`))))) _manacost) 0)
          (bind _success (`/Game/Framework/Blueprints/Abilities/Base/BP_BaseAbility.StartCast` _localability))
          (`self.E_AbilityUsed` _localability)
          (return _success)
          (else
            (`KismetSystemLibrary.PrintString` "Use Ability Failed: InsufficientMana")
            (`self.E_FailedNotEnoughMana` (`local.LocalAbility`))
            (return false)))))
    (:`Is Not Valid`
      (return false))))