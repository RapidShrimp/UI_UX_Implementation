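; Equipment component that tracks a character's equipped items and swaps them with the owner's BPCInventory.
; EquipItem takes the item out of inventory, unequips any item in the same equipment slot, then adds the new one.
; RemoveItem returns an item to inventory only if an empty slot exists, and both paths signal an equipment refresh on success.
; UpdateCurrentWeapon caches and returns the BP_BaseWeapon found in the first slot type.
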(fn `EquipItem`
  (params (ItemToEquip :type "/Game/Framework/Blueprints/Items/Equipment/Base/BP_BaseEquipment Object Reference"))
  (returns (`Success?` :type Boolean))
  (locals (LocalTempItem :type "/Game/Framework/Blueprints/Items/Equipment/Base/BP_BaseEquipment Object Reference") (LocalTempEquipmentSlot :type "/Game/Framework/Blueprints/Data/Items/Enum_EquipmentSlots Enum" :default "NewEnumerator0") (LocalReplaceItem :type Boolean) (LocalItemToReplace :type "/Game/Framework/Blueprints/Items/Equipment/Base/BP_BaseEquipment Object Reference"))
  (bind _bpc_inventory (`/Game/Framework/Blueprints/Characters/BP_BaseCharacter.BPC_Inventory` (`self.Owning Character`)))
  (bind _output_get (set `local.LocalTempItem` ItemToEquip))
  (set `local.LocalTempEquipmentSlot` (`/Game/Framework/Blueprints/Items/Equipment/Base/BP_BaseEquipment.EquipmentSlot` _output_get))
  (for _array_element (`self.EquippedItems`)
    (if (`|EnumEquality` (`/Game/Framework/Blueprints/Items/Equipment/Base/BP_BaseEquipment.EquipmentSlot` _array_element) (`local.LocalTempEquipmentSlot`))
      (set `local.LocalReplaceItem` true)
      (set `local.LocalItemToReplace` _array_element)
      (break)))
  (bind (_foundindex _success_) (`/Game/Framework/Blueprints/Components/BPC_Inventory.FindItemClassIndex` _bpc_inventory (`GameplayStatics.GetObjectClass` (`local.LocalTempItem`))))
  (if _success_
    (`/Game/Framework/Blueprints/Components/BPC_Inventory.RemoveItemAtIndex` _bpc_inventory _foundindex 1)
    (if (`local.LocalReplaceItem`)
      (bind _success__2 (`self.RemoveItem` (`local.LocalItemToReplace`)))
      (if _success__2
        _
        (else
          (return false))))
    (`KismetArrayLibrary.Array_AddUnique` (`self.EquippedItems`) (`local.LocalTempItem`))
    (`self.E_EquipmentRefreshed`)
    (return true)))

(fn `Initialise`
  (params (OwningCharacter :type "/Game/Framework/Blueprints/Characters/BP_BaseCharacter Object Reference"))
  (set `self.Owning Character` OwningCharacter))

(fn `RemoveItem`
  (params (ItemToRemove :type "/Game/Framework/Blueprints/Items/Equipment/Base/BP_BaseEquipment Object Reference"))
  (returns (`Success?` :type Boolean))
  (locals (LocalTempItem :type "/Game/Framework/Blueprints/Items/Equipment/Base/BP_BaseEquipment Object Reference"))
  (bind _localtempitem (`local.LocalTempItem`))
  (bind _bpc_inventory (`/Game/Framework/Blueprints/Characters/BP_BaseCharacter.BPC_Inventory` (`self.Owning Character`)))
  (set `local.LocalTempItem` ItemToRemove)
  (bind _success_ (`/Game/Framework/Blueprints/Components/BPC_Inventory.FindEmptySlot` _bpc_inventory))
  (if _success_
    (`KismetArrayLibrary.Array_RemoveItem` (`self.EquippedItems`) _localtempitem)
    (set `/Game/Framework/Blueprints/Items/Equipment/Base/BP_BaseEquipment.Equipped?` false _localtempitem)
    (`/Game/Framework/Blueprints/Components/BPC_Inventory.AddItem` _bpc_inventory (`GameplayStatics.GetObjectClass` (`local.LocalTempItem`)) 1)
    (`self.E_EquipmentRefreshed`)
    (return true)
    (else
      (return false))))

(fn `UpdateCurrentWeapon`
  (returns (EquippedWeapon :type "/Game/Framework/Blueprints/Items/Equipment/Base/BP_BaseWeapon Object Reference"))
  (set `self.CurrentWeapon` null)
  (for _array_element (`self.EquippedItems`)
    (if (`|EnumEquality` (`/Game/Framework/Blueprints/Items/Equipment/Base/BP_BaseEquipment.EquipmentSlot` _array_element) "NewEnumerator0")
      (bind _asbp_base_weapon (cast `/Game/Framework/Blueprints/Items/Equipment/Base/BP_BaseWeapon` _array_element))
      (set `self.CurrentWeapon` _asbp_base_weapon)
      (break)))
  (return (`self.CurrentWeapon`)))