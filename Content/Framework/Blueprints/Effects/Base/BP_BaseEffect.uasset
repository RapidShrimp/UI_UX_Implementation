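; Base effect Blueprint that manages the stacks and duration of a status effect on an owning character, driven by an EffectData struct.
; AddStack increments stacks below the maximum, then clears the timer and calls StartEffect again.
; StartEffect sets a one-shot timer for non-zero durations.
; EndEffect fires the EEndEffect dispatcher; both start and end print debug messages.
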(fn `AddStack`
  (bind ((`CurrentStacks_11_BBF8139C4FD732DB7A7372B6F2A7086A` _currentstacks) (`MaxStacks_12_C50C44464FCB82E4466CE6ABC5951F0F` _maxstacks)) (break `/Game/Framework/Blueprints/Data/Effects/Struct_EffectData` (`self.EffectData`)))
  (if (< _currentstacks _maxstacks)
    (bind _result (`/Engine/EditorBlueprintResources/StandardMacros.IncrementInt` _currentstacks)
      (:`  `
        (setmembers `/Game/Framework/Blueprints/Data/Effects/Struct_EffectData` :`StructRef` (`self.EffectData`) :`CurrentStacks` _result)
        (`KismetSystemLibrary.K2_ClearAndInvalidateTimerHandle` (`self.EffectTimer`))
        (`self.StartEffect`)
        (return)))))

(fn `EndEffect`
  (bind ((`EffectName_2_D6DC489244E527F5002982B905FED353` _effectname) (`EffectType_14_037EC23F468B25787FD3A099EFBF03B2` _effecttype)) (break `/Game/Framework/Blueprints/Data/Effects/Struct_EffectData` (`self.EffectData`)))
  (`KismetSystemLibrary.PrintString` (`KismetStringLibrary.Concat_StrStr` (`|GetEnumeratorNameAsString` _effecttype) " '" (`KismetStringLibrary.Conv_NameToString` _effectname) "' ended") true true (struct :`R` 1.0 :`B` 0.982251 :`A` 1.0))
  (`self.E_EndEffect` self)
  (return))

(fn `Initialise`
  (params (OwningCharacter :type "/Game/Framework/Blueprints/Characters/BP_BaseCharacter Object Reference"))
  (set `self.Owning Character` OwningCharacter))

(fn `StartEffect`
  (bind ((`EffectName_2_D6DC489244E527F5002982B905FED353` _effectname) (`EffectType_14_037EC23F468B25787FD3A099EFBF03B2` _effecttype)) (break `/Game/Framework/Blueprints/Data/Effects/Struct_EffectData` (`self.EffectData`)))
  (bind ((`EffectDuration_17_B620328D485C1348282DEAB44213DA33` _effectduration)) (break `/Game/Framework/Blueprints/Data/Effects/Struct_EffectData` (`self.EffectData`)))
  (`KismetSystemLibrary.PrintString` (`KismetStringLibrary.Concat_StrStr` (`|GetEnumeratorNameAsString` _effecttype) " '" (`KismetStringLibrary.Conv_NameToString` _effectname) "' started") true true (struct :`R` 1.0 :`B` 0.982251 :`A` 1.0))
  (if (not (== _effectduration 0.0))
    (bind _returnvalue (`KismetSystemLibrary.K2_SetTimerDelegate` (`|CreateDelegate` :!event `EndEffect`) _effectduration))
    (set `self.EffectTimer` _returnvalue)
    (return)))

(fn `UserConstructionScript`)