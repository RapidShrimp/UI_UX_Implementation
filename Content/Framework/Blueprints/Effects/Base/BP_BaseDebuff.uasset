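; Base debuff effect that temporarily lowers one attribute on its owning character.
; StartEffect runs the parent logic, then subtracts ModifierStrength from the AttributeBonus of AffectedAttribute in the character's BPCAttributes component.
; EndEffect runs the parent logic, then adds the same ModifierStrength variable back to undo the penalty.
; Both write directly into the attribute struct array, then call EAttributesModified on the component to signal the change.
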(fn `EndEffect`
  (bind _bpc_attributes (`/Game/Framework/Blueprints/Characters/BP_BaseCharacter.BPC_Attributes` (`self.Owning Character`)))
  (bind _characterattributes_attributes (break `/Game/Framework/Blueprints/Data/Attributes/Struct_CharacterAttributeData` (`/Game/Framework/Blueprints/Components/BPC_Attributes.CharacterAttributes` _bpc_attributes)))
  (bind _output (`|GetArrayItem` _characterattributes_attributes (`/Game/Framework/Blueprints/Components/BPC_Attributes.GetAttributeIndex` _bpc_attributes (`self.AffectedAttribute`))))
  (`parent.EndEffect`)
  (setmembers `/Game/Framework/Blueprints/Data/Attributes/Struct_AttributeData` :`StructRef` _output :`AttributeBonus` (+ (`.AttributeBonus_28_0A1DF031411FB0BBE8A161BD07DBB6E1` (break `/Game/Framework/Blueprints/Data/Attributes/Struct_AttributeData` _output)) (`self.ModifierStrength`)))
  (`/Game/Framework/Blueprints/Components/BPC_Attributes.E_AttributesModified` _bpc_attributes))

(fn `StartEffect`
  (bind _bpc_attributes (`/Game/Framework/Blueprints/Characters/BP_BaseCharacter.BPC_Attributes` (`self.Owning Character`)))
  (bind _characterattributes_attributes (break `/Game/Framework/Blueprints/Data/Attributes/Struct_CharacterAttributeData` (`/Game/Framework/Blueprints/Components/BPC_Attributes.CharacterAttributes` _bpc_attributes)))
  (bind _output (`|GetArrayItem` _characterattributes_attributes (`/Game/Framework/Blueprints/Components/BPC_Attributes.GetAttributeIndex` _bpc_attributes (`self.AffectedAttribute`))))
  (`parent.StartEffect`)
  (setmembers `/Game/Framework/Blueprints/Data/Attributes/Struct_AttributeData` :`StructRef` _output :`AttributeBonus` (- (`.AttributeBonus_28_0A1DF031411FB0BBE8A161BD07DBB6E1` (break `/Game/Framework/Blueprints/Data/Attributes/Struct_AttributeData` _output)) (`self.ModifierStrength`)))
  (`/Game/Framework/Blueprints/Components/BPC_Attributes.E_AttributesModified` _bpc_attributes))

(fn `UserConstructionScript`
  (`parent.UserConstructionScript`))