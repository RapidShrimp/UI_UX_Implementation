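; BP_BaseProjectile is a base projectile actor that damages what it hits and then removes itself.
; BeginPlay sets the actor's lifespan from the Lifespan variable, which can be set on spawn.
; A CollisionSphere hit on anything but the owner applies ProjectileDamage, with the instigator as damage causer.
; The hit then calls HandleDeath, a separate function that only destroys the actor.
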(event `DefineLifespan`
  ;[0 0 0] Define the Lifespan of the Projectile -
  ; Change the Lifespan Variable
  (`self.SetLifeSpan` self (`self.Lifespan`)))

(event `self.ReceiveBeginPlay`
  ;[0 0 0] Projectile Begin Play - Define Lifespan - Can be defined on Spawn
  (`self.DefineLifespan`))

(event `self.CollisionSphere.OnComponentHit`
  (params (HitComponent :type "PrimitiveComponent Object Reference") (OtherActor :type "Actor Object Reference") (OtherComp :type "PrimitiveComponent Object Reference") (NormalImpulse :type "Vector Structure") (Hit :type "HitResult Structure (by ref)"))
  ;[0 0 0] On Collision with another Actor - Apply Damage to them and then Handle Death for this Projectile
  (if (!= OtherActor (`self.GetOwner`))
    (`GameplayStatics.ApplyDamage` OtherActor (`self.ProjectileDamage`) (`self.GetInstigatorController` (`self.Instigator`)) (`self.GetInstigator`))
    (`self.HandleDeath`)))

(fn `HandleDeath`
  (`self.K2_DestroyActor`))

(fn `UserConstructionScript`)