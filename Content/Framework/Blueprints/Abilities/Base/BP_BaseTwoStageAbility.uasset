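; BP_BaseTwoStageAbility is a base ability Blueprint that adds a pre-cast stage before the normal cast.
; StartCast refuses while on cooldown; otherwise the first call runs PreCastExecute, which sets PreCasting and calls the EPreCast event.
; A second call while PreCasting hands off to the parent StartCast.
; Executing or interrupting the ability runs the parent logic and clears PreCasting.
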(fn `ExecuteAbility`
  (`parent.ExecuteAbility`)
  (set `self.PreCasting` false)
  (return))

(fn `InterruptAbility`
  (`parent.InterruptAbility`)
  (set `self.PreCasting` false)
  (return))

(fn `PreCastExecute`
  (returns (Success :type Boolean))
  (set `self.PreCasting` true)
  (`KismetSystemLibrary.PrintString` "PreCasting" true true (struct :`R` 1.0 :`G` 0.502887 :`A` 1.0))
  (`self.E_PreCast`)
  (return false))

(fn `StartCast`
  (returns (Success :type Boolean))
  (if (`.OnCooldown_14_05A44E6C4479C8C6DD247DB54A60EB4A` (break `/Game/Framework/Blueprints/Data/Ability/Struct_AbilityData` (`self.AbilityData`)))
    (`KismetSystemLibrary.PrintString` "Use Ability Failed: On Cooldown" true true (struct :`R` 1.0 :`G` 0.502887 :`A` 1.0))
    (return false)
    (elif (`self.PreCasting`)
      (bind _success (`parent.StartCast`))
      (return _success)
      (else
        (`self.PreCastExecute`)
        (return true)))))

(fn `UserConstructionScript`
  (`parent.UserConstructionScript`))