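; Base area-of-effect ability that applies effects to characters within the ability's AOE range around the owning character.
; On execution, a multi-sphere object trace at the owner's location picks object types by friendly, hostile or unset targeting, without ignoring self.
; Each hit BP_BaseCharacter receives EffectsToAdd through its effects component, and each such hit triggers the owner's ranged attack animation.
; Debug spheres visualize the radius.
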(fn `ExecuteAbility`
  (bind _owning_character (`self.Owning Character`))
  (bind ((`AOERange_33_609922A14C1F975257DD38AD80786627` _aoerange)) (break `/Game/Framework/Blueprints/Data/Ability/Struct_AbilityData` (`self.AbilityData`)))
  (bind _returnvalue (`self.K2_GetActorLocation` (`self.Owning Character`)))
  (`parent.ExecuteAbility`)
  (`KismetSystemLibrary.DrawDebugSphere` _returnvalue _aoerange 12 (struct :`R` 1.0 :`G` 0.502887 :`A` 1.0) 0.5 2.0)
  (bind (_outhits _returnvalue_2) (`KismetSystemLibrary.SphereTraceMultiForObjects` :`Start` _returnvalue :`End` _returnvalue :`Radius` _aoerange :`ObjectTypes` (select `/Game/Framework/Blueprints/Data/Attributes/Enum_HostileState` (`self.EnumHostile`) :`NewEnumerator0` (`|MakeArray` "ObjectTypeQuery7" "ObjectTypeQuery9" :!type "EObjectTypeQuery Enum") :`NewEnumerator1` (`|MakeArray` "ObjectTypeQuery9" :!type "EObjectTypeQuery Enum") :`NewEnumerator2` (`|MakeArray` "ObjectTypeQuery7" :!type "EObjectTypeQuery Enum")) :`DrawDebugType` "ForDuration" :`bIgnoreSelf` false))
  (if _returnvalue_2
    (for _array_element _outhits
      (bind _asbp_base_character (cast `/Game/Framework/Blueprints/Characters/BP_BaseCharacter` (`.HitActor` (`GameplayStatics.BreakHitResult` _array_element))))
      (`/Game/Framework/Blueprints/Components/BPC_Effects.Add Effect` (`/Game/Framework/Blueprints/Characters/BP_BaseCharacter.BPC_Effects` _asbp_base_character) (`self.Effects to Add`))
      (set `/Game/Framework/Blueprints/Characters/BP_BaseCharacter.IsUsingRangedAttack` true _owning_character)
      (`/Game/Framework/Blueprints/Characters/BP_BaseCharacter.PlayAttackAnim` _owning_character))))

(fn `UserConstructionScript`
  (`parent.UserConstructionScript`))