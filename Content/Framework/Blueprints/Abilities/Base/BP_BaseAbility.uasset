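; Base ability Actor that manages the cast, execution, interruption and cooldown cycle of an ability for its owning character.
; Initialise stores owner and ID, UseAbility forwards that ID to the owner's BPCAbilities component, and StartCast starts a cast timer.
; Execution and interruption both start the cooldown, while ResetAbility clears it and notifies the component.
; Event dispatchers broadcast execution with mana cost, widget cooldown, interruption and cooldown completion.
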(fn `ExecuteAbility`
  (bind _abilitydata (`self.AbilityData`))
  (bind ((`AbilityName_3_6E6EB55842ABB698C00E9A9845F1E1DF` _abilityname) (`CooldownTime_6_043A697942E5CF2F1B0C2DA03D43FA86` _cooldowntime) (`ManaCost_9_ED8622F44C9BB2B067A4AEB193B018C4` _manacost)) (break `/Game/Framework/Blueprints/Data/Ability/Struct_AbilityData` _abilitydata))
  (bind _returnvalue (`KismetSystemLibrary.K2_SetTimerDelegate` (`|CreateDelegate` :!event `ResetAbility`) _cooldowntime))
  (set `self.CooldownTimer` _returnvalue)
  (setmembers `/Game/Framework/Blueprints/Data/Ability/Struct_AbilityData` :`StructRef` _abilitydata :`OnCooldown` true)
  (`KismetSystemLibrary.PrintString` (`KismetStringLibrary.Concat_StrStr` "Ability used: " (`KismetStringLibrary.Conv_NameToString` _abilityname)) true true (struct :`R` 1.0 :`G` 0.502887 :`A` 1.0))
  (`self.E_ExecuteAbility` _manacost)
  (`self.E_WidgetCooldown`))

(fn `Initialise`
  (params (OwningCharacter :type "/Game/Framework/Blueprints/Characters/BP_BaseCharacter Object Reference") (AbilityID :type Integer))
  (set `self.Owning Character` OwningCharacter)
  (setmembers `/Game/Framework/Blueprints/Data/Ability/Struct_AbilityData` :`StructRef` (`self.AbilityData`) :`AbilityID` AbilityID))

(fn `InterruptAbility`
  (bind _abilitydata (`self.AbilityData`))
  (setmembers `/Game/Framework/Blueprints/Data/Ability/Struct_AbilityData` :`StructRef` _abilitydata :`OnCooldown` true)
  (bind _returnvalue (`KismetSystemLibrary.K2_SetTimerDelegate` (`|CreateDelegate` :!event `ResetAbility`) (`.CooldownTime_6_043A697942E5CF2F1B0C2DA03D43FA86` (break `/Game/Framework/Blueprints/Data/Ability/Struct_AbilityData` _abilitydata))))
  (set `self.CooldownTimer` _returnvalue)
  (`self.E_Interrupted`))

(fn `ResetAbility`
  (`KismetSystemLibrary.K2_ClearAndInvalidateTimerHandle` (`self.CooldownTimer`))
  (`/Game/Framework/Blueprints/Components/BPC_Abilities.AbilityCooledDown` (`/Game/Framework/Blueprints/Characters/BP_BaseCharacter.BPC_Abilities` (`self.Owning Character`)) self)
  (`self.E_CooldownFinished`)
  (setmembers `/Game/Framework/Blueprints/Data/Ability/Struct_AbilityData` :`StructRef` (`self.AbilityData`) :`OnCooldown` false))

(fn `StartCast`
  (returns (Success :type Boolean))
  (`KismetSystemLibrary.K2_SetTimerDelegate` (`|CreateDelegate` :!event `ExecuteAbility`) (`.CastTime_26_76BE4CE141E81392457977AC49ABE8BE` (break `/Game/Framework/Blueprints/Data/Ability/Struct_AbilityData` (`self.AbilityData`))))
  (return true))

(fn `UseAbility`
  (`/Game/Framework/Blueprints/Components/BPC_Abilities.UseAbility` (`/Game/Framework/Blueprints/Characters/BP_BaseCharacter.BPC_Abilities` (`self.Owning Character`)) (`.AbilityID_11_077042614950DBE0C3BD528FCEDE28D5` (break `/Game/Framework/Blueprints/Data/Ability/Struct_AbilityData` (`self.AbilityData`)))))

(fn `UserConstructionScript`)