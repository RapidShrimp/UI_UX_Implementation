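; Base Blueprint for skill-shot abilities, which the player aims with the mouse cursor and which fire a projectile.
; On initialise it attaches to the owning character at the capsule's base with its aiming decal hidden.
; During pre-cast, a looping timer traces under the cursor, turning the decal and character toward the hit point.
; Execution stops the timer, spawns the projectile at the character's FirePoint along that yaw, then refreshes the aim state.
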(fn `ExecuteAbility`
  (bind _owning_character (`self.Owning Character`))
  (`KismetSystemLibrary.K2_ClearAndInvalidateTimerHandle` (`self.AimRefreshTimer`))
  (`parent.ExecuteAbility`)
  (`|SpawnActorFromClass` (`self.SpawnedProjectile`) (`KismetMathLibrary.MakeTransform` (`SceneComponent.K2_GetComponentLocation` (`/Game/Framework/Blueprints/Characters/BP_BaseCharacter.FirePoint` (`self.Owning Character`))) (`KismetMathLibrary.MakeRotator` 0.0 0.0 (`self.YawDir`))) "Undefined" "OverrideRootScale" _owning_character _owning_character)
  (`self.UpdateAim`))

(fn `Initialise`
  (params (OwningCharacter :type "/Game/Framework/Blueprints/Characters/BP_BaseCharacter Object Reference") (AbilityID :type Integer))
  (`parent.Initialise` OwningCharacter AbilityID)
  (`self.K2_AttachToActor` self (`local.OwningCharacter`) "None" "SnapToTarget" "KeepWorld" "KeepWorld" true)
  (`self.K2_SetActorRelativeLocation` (`KismetMathLibrary.MakeVector` 0.0 0.0 (* (`CapsuleComponent.GetScaledCapsuleHalfHeight` (`Character.CapsuleComponent` (`local.OwningCharacter`))) -1.0)))
  (`SceneComponent.SetHiddenInGame` (`self.AimingDecal`) true false)
  (`self.EnableInput` (`GameplayStatics.GetPlayerController` 0)))

(fn `PreCastExecute`
  (returns (Success :type Boolean))
  (bind _success (`parent.PreCastExecute`))
  (bind _returnvalue (`KismetSystemLibrary.K2_SetTimer` null "UpdateAim" 0.01 true))
  (set `self.AimRefreshTimer` _returnvalue)
  (return _success))

(fn `UpdateAim`
  (bind (_returnvalue_roll _returnvalue_pitch _returnvalue_yaw) (`KismetMathLibrary.BreakRotator` (`KismetMathLibrary.FindLookAtRotation` (`self.K2_GetActorLocation` (`self.Owning Character`)) (`.Location` (`GameplayStatics.BreakHitResult` (`PlayerController.GetHitResultUnderCursorByChannel` (`GameplayStatics.GetPlayerController` 0) "TraceTypeQuery1" true))))))
  (if (`self.PreCasting`)
    (`SceneComponent.SetHiddenInGame` (`self.AimingDecal`) false false)
    (bind _output_get (set `self.YawDir` _returnvalue_yaw))
    (`self.K2_SetActorRotation` (`KismetMathLibrary.MakeRotator` 0.0 0.0 _output_get))
    (`self.K2_SetActorRotation` (`self.Owning Character`) (`KismetMathLibrary.MakeRotator` 0.0 0.0 _returnvalue_yaw) false)
    (return)
    (else
      (set `self.YawDir` 0.0)
      (`SceneComponent.SetHiddenInGame` (`self.AimingDecal`) true false)
      (return))))

(fn `UserConstructionScript`
  (`parent.UserConstructionScript`))