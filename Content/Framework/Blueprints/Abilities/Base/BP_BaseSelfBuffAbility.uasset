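; BP_BaseSelfBuffAbility is a base ability Blueprint for buffs that apply an effect to the character that owns the ability.
; ExecuteAbility runs the parent implementation, then passes EffectToAdd to the owning character's BPCEffects component through AddEffect.
; The event graph holds only disabled stub events, so all of its own behavior lives in that override.
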(fn `ExecuteAbility`
  (`parent.ExecuteAbility`)
  (`/Game/Framework/Blueprints/Components/BPC_Effects.Add Effect` (`/Game/Framework/Blueprints/Characters/BP_BaseCharacter.BPC_Effects` (`self.Owning Character`)) (`self.EffectToAdd`)))

(fn `UserConstructionScript`
  (`parent.UserConstructionScript`))