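; Base area-of-effect damage ability that strikes around its owning character when executed.
; It extends the parent ability's execution and applies radial damage at the owner's location using the damage and range from its ability data, crediting the owner and its controller.
; It also draws a brief debug sphere for the radius, flags the owner as using a ranged attack, and plays the owner's attack animation.
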(fn `ExecuteAbility`
  (bind _owning_character (`self.Owning Character`))
  (bind ((`DamageAmount_32_B37A0CA749E235BD5B652B8F94A10190` _damageamount) (`AOERange_33_609922A14C1F975257DD38AD80786627` _aoerange)) (break `/Game/Framework/Blueprints/Data/Ability/Struct_AbilityData` (`self.AbilityData`)))
  (bind _returnvalue (`self.K2_GetActorLocation` _owning_character))
  (`parent.ExecuteAbility`)
  (`KismetSystemLibrary.DrawDebugSphere` _returnvalue (`.AOERange_33_609922A14C1F975257DD38AD80786627` (break `/Game/Framework/Blueprints/Data/Ability/Struct_AbilityData` (`self.AbilityData`))) 12 (struct :`R` 1.0 :`G` 0.502887 :`A` 1.0) 0.5 2.0)
  (`GameplayStatics.ApplyRadialDamage` :`BaseDamage` _damageamount :`Origin` _returnvalue :`DamageRadius` _aoerange :`DamageCauser` _owning_character :`InstigatedByController` (`Pawn.GetController` _owning_character))
  (set `/Game/Framework/Blueprints/Characters/BP_BaseCharacter.IsUsingRangedAttack` true _owning_character)
  (`/Game/Framework/Blueprints/Characters/BP_BaseCharacter.PlayAttackAnim` _owning_character))

(fn `UserConstructionScript`
  (`parent.UserConstructionScript`))